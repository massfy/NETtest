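; Player controller for battle matches that drives player list, match start and end-of-game UI.
; CreatePlayerInfo adds a PlayerState to the PlayerList widget, and ShowOtherPlayerUI calls InitPlayers on the controlled BP_BattleCharacter.
; WaitToStart and ReadyPlay signal through "ce" console commands, which target level Blueprint events.
; GameWin and GameLose remove all widgets, clear the character's sprint and health timers, then show the winner or loser screen.
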(event `CreatePlayerInfo`
  (params (PlayerState :type "BattlePlayerState Object Reference"))
  (bind _asplayer_list (cast `/Game/UI/PlayerList` (`self.PlayerListWidget`)))
  (`/Game/UI/PlayerList.AddPlayer` _asplayer_list PlayerState))

(event `WaitToStart`
  (`KismetSystemLibrary.ExecuteConsoleCommand` "ce ShowWaitUI" null))

(event `ReadyPlay`
  (`KismetSystemLibrary.ExecuteConsoleCommand` "ce ReadyPlay" null))

(event `ShowOtherPlayerUI`
  (bind _asbp_battle_character (cast `/Game/Characters/BP_BattleCharacter` (`self.K2_GetPawn`)))
  (`/Game/Characters/BP_BattleCharacter.InitPlayers` _asbp_battle_character))

(event `GameWin`
  (`self.ClearTimerAndWidget`)
  (bind _returnvalue (`|CreateWidget` "/Game/UI/WinnerUI.WinnerUI_C" self))
  (`UserWidget.AddToViewport` _returnvalue 0))

(event `GameLose`
  (`self.ClearTimerAndWidget`)
  (bind _returnvalue (`|CreateWidget` "/Game/UI/GameLose.GameLose_C"))
  (`UserWidget.AddToViewport` _returnvalue 0))

(event `ClearTimerAndWidget`
  (`WidgetLayoutLibrary.RemoveAllWidgets`)
  (bind _asbp_battle_character (cast `/Game/Characters/BP_BattleCharacter` (`self.K2_GetPawn`)))
  (`KismetSystemLibrary.K2_ClearAndInvalidateTimerHandle` (`BattleCharacter.MySprintTimerHandle` _asbp_battle_character))
  (`KismetSystemLibrary.K2_ClearAndInvalidateTimerHandle` (`BattleCharacter.HealthTimerHandle` _asbp_battle_character)))

(fn `UserConstructionScript`)