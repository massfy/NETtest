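; Battle game instance that handles multiplayer session hosting, browsing and joining, with a shared UseLAN setting for hosting and searching.
; CreateSession requests a fixed-size session, then stores MaxPlayerNum and opens GameMap as a listen server; the stored value does not size the session.
; FindSession adds a SessionItem widget per result to the supplied container.
; JoinSession shows the session-full popup on any join failure.
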(event `CreateSession`
  (params (MaxPlayerNum :type Integer))
  ;[1 1 1] CreateSession
  (`CreateSessionCallbackProxy.CreateSession` (`GameplayStatics.GetPlayerController` 0) 100 (`self.UseLAN?`)
    (:`OnSuccess`
      (set `self.MaxPlayerNum` MaxPlayerNum)
      (`GameplayStatics.OpenLevel` "GameMap" true "listen"))))

(event `FindSession`
  (params (`目标` :type "PanelWidget Object Reference"))
  (bind _returnvalue (`GameplayStatics.GetPlayerController` 0))
  ;[1 1 1] FindSession
  (bind _results (`FindSessionsCallbackProxy.FindSessions` _returnvalue 100 (`self.UseLAN?`))
    (:`OnSuccess`
      (for _array_element _results
        (bind _returnvalue_2 (`|CreateWidget` "/Game/UI/Sessions/SessionItem.SessionItem_C" _returnvalue (`FindSessionsCallbackProxy.GetServerName` _array_element) _array_element))
        (`PanelWidget.AddChild` `目标` _returnvalue_2)))))

(event `JoinSession`
  (params (SearchResult :type "BlueprintSessionResult Structure (by ref)"))
  ;[1 1 1] JoinSessiom
  (`JoinSessionCallbackProxy.JoinSession` (`GameplayStatics.GetPlayerController` 0) SearchResult
    (:`OnFailure`
      (bind _returnvalue (`|CreateWidget` "/Game/UI/Sessions/SessionPlayerNumIsFull.SessionPlayerNumIsFull_C" (`GameplayStatics.GetPlayerController` 0)))
      (`UserWidget.AddToViewport` _returnvalue 0))))