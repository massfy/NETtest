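; BP_DeathActor is a character death actor that plays a death animation in a body color.
; On BeginPlay it passes its source material and BodyColor to SetMaterialOnServer, then plays the non-looping Death_1 animation on its mesh.
; SetMaterialOnServer forwards to SetMaterialToAll, a server-to-all naming pattern, which creates a dynamic material instance on the mesh and sets a vector parameter to the color.
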(event `self.ReceiveBeginPlay`
  ;[1 1 1] BeginPlay
  (`self.SetMaterialOnServer` 0 (`self.SourceMaterial`) "BodyColor" (`self.BodyColor`))
  (`SkeletalMeshComponent.PlayAnimation` (`self.Mesh`) "/Game/Mannequin/Animations/Death_1.Death_1" false))

(event `SetMaterialOnServer`
  (params (ElementIndex :type Integer) (SourceMaterial :type "MaterialInterface Object Reference") (ParameterName :type Name :default "BodyColor") (Value :type "LinearColor Structure"))
  (`self.SetMaterialToAll` ElementIndex SourceMaterial ParameterName Value))

(event `SetMaterialToAll`
  (params (ElementIndex :type Integer) (SourceMaterial :type "MaterialInterface Object Reference") (ParameterName :type Name :default "BodyColor") (Value :type "LinearColor Structure"))
  (bind _returnvalue (`PrimitiveComponent.CreateDynamicMaterialInstance` (`self.Mesh`) ElementIndex SourceMaterial "None"))
  (`MaterialInstanceDynamic.SetVectorParameterValue` _returnvalue ParameterName Value))

(fn `UserConstructionScript`)